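; Controller that drives a BP_CarPawn around a looping list of checkpoints taken from the pawn, with simple obstacle avoidance.
; Each tick it moves the car forward and runs a box trace, turning right while blocked, otherwise rotating smoothly toward the current checkpoint.
; Arrival is a distance test that advances and wraps the checkpoint index, printing it for debug.
; StartAndCheckAvoidance is an unfinished, uncalled stub.
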(event `self.ReceiveBeginPlay`
  (bind _asbp_car_pawn (cast `/Game/BP_Playground/BP_CarPawn` (`self.K2_GetPawn`)))
  (bind _output_get (set `self.ControlledCar` _asbp_car_pawn))
  (bind _output_get_2 (set `self.Checkpoints` (`/Game/BP_Playground/BP_CarPawn.Checkpoints` _output_get)))
  (set `self.CurrentMovementTargetLocation` (`self.K2_GetActorLocation` (`|GetArrayItem` _output_get_2 (`self.CheckPointCurrentIndex`)))))

(event `self.ReceiveTick`
  (params (DeltaSeconds :type "Float (single-precision)"))
  (bind _controlledcar (`self.ControlledCar`))
  (`/Game/BP_Playground/BP_CarPawn.MoveForwardByTick` _controlledcar DeltaSeconds)
  (`/Game/BP_Playground/BP_CarPawn.TraceBoxObstacleDetection` _controlledcar)
  (if (`/Game/BP_Playground/BP_CarPawn.ObstacleDetected` _controlledcar)
    (`/Game/BP_Playground/BP_CarPawn.TurnRightByTick` _controlledcar DeltaSeconds)
    (else
      (`/Game/BP_Playground/BP_CarPawn.SmoothRotateToTarget` _controlledcar DeltaSeconds (`self.CurrentMovementTargetLocation`))
      (`self.CheckTargetApproach`))))

(fn `CheckTargetApproach`
  (bind _controlledcar (`self.ControlledCar`))
  (if (<= (`KismetMathLibrary.Vector_Distance` (`self.K2_GetActorLocation` _controlledcar) (`self.CurrentMovementTargetLocation`)) (`/Game/BP_Playground/BP_CarPawn.ArrivalConfirmationDistance` _controlledcar))
    (bind _result (`/Engine/EditorBlueprintResources/StandardMacros.IncrementInt` (`self.CheckPointCurrentIndex`))
      (:`  `
        (bind _output_get (set `self.CheckPointCurrentIndex` (mod _result (`KismetArrayLibrary.Array_Length` (`self.Checkpoints`)))))
        (`KismetSystemLibrary.PrintString` (`KismetStringLibrary.Conv_IntToString` _output_get))
        (set `self.CurrentMovementTargetLocation` (`self.K2_GetActorLocation` (`|GetArrayItem` (`self.Checkpoints`) _output_get)))))))

(fn `StartAndCheckAvoidance`
  (returns (bIsObstacleAvoided :type Boolean))
  (if (`/Game/BP_Playground/BP_CarPawn.ObstacleAvoided` (`self.ControlledCar`))
    _))

(fn `UserConstructionScript`)