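; BP_CarPawn is a car pawn with building blocks for simple movement, steering and obstacle detection.
; Functions drive it along local X at Speed, turn it right at TurningRate, or rotate it toward a target location at constant speed.
; Obstacle detection box-traces from an arrow using the collision box's extents, stores the hit, clears ObstacleAvoided and prints the location.
; Tick and overlap events are empty, so this graph calls none of these functions.
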(event `self.ReceiveTick`
  (params (DeltaSeconds :type "Float (single-precision)")))

(fn `MoveForwardByTick`
  (params (DeltaSeconds :type "Float (double-precision)"))
  (`self.K2_AddActorLocalOffset` (`KismetMathLibrary.MakeVector` (* DeltaSeconds (`self.Speed`)))))

(fn `SmoothRotateToTarget`
  (params (DeltaTime :type "Float (double-precision)") (TargetLocation :type "Vector Structure (by ref)"))
  (`self.K2_SetActorRotation` (`KismetMathLibrary.RInterpTo_Constant` (`self.K2_GetActorRotation`) (`KismetMathLibrary.FindLookAtRotation` (`self.K2_GetActorLocation`) TargetLocation) DeltaTime (`self.TurningRate`))))

(fn `TraceBoxObstacleDetection`
  (bind _arrow (`self.Arrow`))
  (bind _returnvalue (`SceneComponent.K2_GetComponentLocation` _arrow))
  (bind (_returnvalue_x _returnvalue_y _returnvalue_z) (`KismetMathLibrary.BreakVector` (`BoxComponent.GetScaledBoxExtent` (`self.Box`))))
  (bind (_outhit _returnvalue_2) (`KismetSystemLibrary.BoxTraceSingle` :`Start` _returnvalue :`End` (+ _returnvalue (* (`SceneComponent.GetForwardVector` _arrow) (`self.SpottingDistance`))) :`HalfSize` (`KismetMathLibrary.MakeVector` _returnvalue_y _returnvalue_x _returnvalue_z) :`Orientation` (`self.K2_GetActorRotation`) :`TraceChannel` "TraceTypeQuery1" :`DrawDebugType` "ForDuration" :`DrawTime` 0.0))
  (bind _output_get (set `self.TraceResults` _outhit))
  (bind _output_get_2 (set `self.ObstacleDetected` _returnvalue_2))
  (if _output_get_2
    (set `self.ObstacleAvoided` false)
    (`KismetSystemLibrary.PrintString` (`KismetStringLibrary.Conv_VectorToString` (`.Location` (`GameplayStatics.BreakHitResult` _output_get))))
    (return)))

(fn `TurnRightByTick`
  (params (DeltaTime :type "Float (double-precision)"))
  (`self.K2_AddActorLocalRotation` (`KismetMathLibrary.MakeRotator` 0.0 0.0 (* DeltaTime (`self.TurningRate`)))))

(fn `UserConstructionScript`)